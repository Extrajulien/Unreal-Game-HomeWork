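; BP_chest is an interactable chest that swings open when the Interact event fires.
; Interact calls Toggle, which, despite its name, only opens: it sets IsOpen, prints a French debug message and calls Open, with no path to close.
; Open plays a timeline that lerps the Pivot component's relative roll to a quarter turn.
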(event Custom|Open
  (bind _alpha (Timeline|Timeline Play)
    (:Update
      (Transformation|SetRelativeRotation (Variables|Default|Getpivot) (Math|Rotator|MakeRotator (Math|Float|Lerp 0.0 -9e+01 _alpha) 0.0 0.0) false false))))

(event EventBeginPlay)

(event Collision|EventActorBeginOverlap
  (params (OtherActor :type Actor%20Object%20Reference)))

(event EventInteract
  (CallFunction|Toggle))

(fn ConstructionScript)

(fn Toggle
  (if (not (Variables|Default|Getis_open))
    (Variables|Default|Setis_open true)
    (Development|PrintString "Coffre ouvert!")
    (CallFunction|Open)))