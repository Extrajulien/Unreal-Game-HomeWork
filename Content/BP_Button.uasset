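; BP_Button is a toggle button that moves another actor, Affected, by a RelativeMove offset when interacted with.
; Each Interact flips IsOn, playing or reversing a timeline that lerps Affected from its BeginPlay location while sinking the button 5 units.
; The assignment of OriginalButtonLocation is unconnected, so the button animates around that variable's stored value rather than its placed position.
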(event EventBeginPlay
  (Variables|Default|Setoriginal_affected_location (Transformation|GetActorLocation (Variables|Default|GetAffected))))

(event Collision|EventActorBeginOverlap
  (params (OtherActor :type Actor%20Object%20Reference)))

(event EventTick
  (params (DeltaSeconds :type Float%20%28single-precision%29)))

(event EventInteract
  (params (caller :type Actor%20Object%20Reference))
  (bind _original_button_location (Variables|Default|Getoriginal_button_location))
  (bind _original_affected_location (Variables|Default|Getoriginal_affected_location))
  (bind _output_get (Variables|Components|Setis_on (not (Variables|Components|Getis_on))))
  (if _output_get
    (bind _alpha (Timeline|Timeline Play)
      (:Update
        (Transformation|SetRelativeLocation (Variables|Default|Getbutton) (Math|Vector|Lerp(Vector) _original_button_location (+ _original_button_location (Math|Vector|MakeVector 0.0 0.0 5.0)) (Math|Float|Lerp 1.0 0.0 _alpha)) false false)
        (Transformation|SetActorLocation (Variables|Default|GetAffected) (Math|Vector|Lerp(Vector) _original_affected_location (+ _original_affected_location (Variables|Default|Getrelative_move)) _alpha) false false)))
    (else
      (Timeline|Timeline Reverse))))

(fn ConstructionScript)